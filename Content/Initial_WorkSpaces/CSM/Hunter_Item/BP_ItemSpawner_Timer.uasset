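; Item spawner that spawns a pickup on BeginPlay and respawns it after a delay once it leaves the detector, with spawning limited to authority.
; Optional random mode uses a weighted roll among three item classes, heavily favoring the first.
; An "Item"-tagged actor leaving the detector starts a self-rearming respawn timer, which is cleared when a tagged item overlaps again.
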(event OnComponentBeginOverlap(ItemDetector)
  (params (OverlappedComponent :type Primitive%20Component%20Object%20Reference) (OtherActor :type Actor%20Object%20Reference) (OtherComp :type Primitive%20Component%20Object%20Reference) (OtherBodyIndex :type Integer) (bFromSweep :type Boolean) (SweepResult :type Hit%20Result%20Structure%20%28by%20ref%29))
  (if (Actor|ActorHasTag OtherActor "Item")
    (Utilities|Time|ClearandInvalidateTimerbyHandle (Variables|Default|GetRespawnTimerHandle))))

(event OnComponentEndOverlap(ItemDetector)
  (params (OverlappedComponent :type Primitive%20Component%20Object%20Reference) (OtherActor :type Actor%20Object%20Reference) (OtherComp :type Primitive%20Component%20Object%20Reference) (OtherBodyIndex :type Integer))
  (if (Actor|ActorHasTag OtherActor "Item")
    (if (Variables|SpawerSet|GetUseRandomSpawn?)
      (CallFunction|SetItemNum))
    (Utilities|FlowControl|Delay (Variables|SpawerSet|GetRespawnDelay))
    (CallFunction|RespawnTimer)))

(event Custom|ServerRespawn
  (Networking|SwitchHasAuthority
    (:Authority
      (CallFunction|Respawn))))

(event Custom|SetItemNum
  (Variables|Default|SetItemNum (Math|Random|RandomIntegerinRange 1 100))
  (if (<= (Variables|Default|GetItemNum) 97)
    (Variables|SpawerSet|SetSetItem (Variables|SpawerSet|GetSetItem_0))
    (elif (<= (Variables|Default|GetItemNum) 99)
      (Variables|SpawerSet|SetSetItem (Variables|SpawerSet|GetSetItem_1))
      (else
        (Variables|SpawerSet|SetSetItem (Variables|SpawerSet|GetSetItem_2))))))

(event Custom|RespawnTimer
  (bind _returnvalue (Utilities|Time|SetTimerbyEvent (delegate Custom|RespawnTimer) (Variables|SpawerSet|GetRespawnDelay)))
  (Variables|Default|SetRespawnTimerHandle _returnvalue)
  (CallFunction|ServerRespawn))

(event EventBeginPlay
  (if (Variables|SpawerSet|GetUseRandomSpawn?)
    (CallFunction|SetItemNum))
  (CallFunction|ServerRespawn))

(fn ConstructionScript)

(fn Respawn
  (Game|SpawnActorfromClass (Variables|SpawerSet|GetSetItem) (Transformation|GetWorldTransform (Variables|Default|GetItem)) "Undefined" 0 0))