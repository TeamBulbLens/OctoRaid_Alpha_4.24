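; Item spawner actor that respawns a pickup at its Item component's transform once the previous one leaves.
; ItemDetector overlaps with "Item"-tagged actors toggle the spawn flag and actor tick, whose interval is set to RespawnDelay.
; While enabled, Tick waits RespawnDelay, then spawns SetItem through an authority-checked event.
; Optional random mode picks SetItem from three weighted tiers, heavily favoring the first, at BeginPlay and whenever an item leaves.
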(event OnComponentBeginOverlap(ItemDetector)
  (params (OverlappedComponent :type Primitive%20Component%20Object%20Reference) (OtherActor :type Actor%20Object%20Reference) (OtherComp :type Primitive%20Component%20Object%20Reference) (OtherBodyIndex :type Integer) (bFromSweep :type Boolean) (SweepResult :type Hit%20Result%20Structure%20%28by%20ref%29))
  ;[1 1 1] Spawn Switch
  (if (Actor|ActorHasTag OtherActor "Item")
    (Variables|Default|SetIsSpawn? false)
    (Actor|Tick|SetActorTickEnabled false)))

(event OnComponentEndOverlap(ItemDetector)
  (params (OverlappedComponent :type Primitive%20Component%20Object%20Reference) (OtherActor :type Actor%20Object%20Reference) (OtherComp :type Primitive%20Component%20Object%20Reference) (OtherBodyIndex :type Integer))
  ;[1 1 1] Spawn Switch
  (if (Actor|ActorHasTag OtherActor "Item")
    (Variables|Default|SetIsSpawn? true)
    (if (Variables|Default|GetUseRandomSpawn)
      (CallFunction|SetItemNum))
    (Actor|Tick|SetActorTickEnabled true)))

(event Custom|ServerSpawnItem
  ;[1 1 1] Item Spawn
  (Networking|SwitchHasAuthority
    (:Authority
      (CallFunction|Respawn))))

(event Custom|SetItemNum
  (Variables|Default|SetItemNum (Math|Random|RandomIntegerinRange 1 100))
  (if (<= (Variables|Default|GetItemNum) 97)
    (Variables|Default|SetSetItem (Variables|Default|GetSetItem_0))
    (elif (<= (Variables|Default|GetItemNum) 99)
      (Variables|Default|SetSetItem (Variables|Default|GetSetItem_1))
      (else
        (Variables|Default|SetSetItem (Variables|Default|GetSetItem_2))))))

(event EventBeginPlay
  (if (Variables|Default|GetUseRandomSpawn)
    (CallFunction|SetItemNum))
  (Actor|Tick|SetActorTickInterval (Variables|Default|GetRespawnDelay)))

(event EventTick
  (params (DeltaSeconds :type Float%20%28single-precision%29))
  ;[1 1 1] Item Spawn
  (if (Variables|Default|GetIsSpawn?)
    (Utilities|FlowControl|Delay (Variables|Default|GetRespawnDelay))
    (CallFunction|ServerSpawnItem)))

(fn ConstructionScript)

(fn Respawn
  (Game|SpawnActorfromClass (Variables|Default|GetSetItem) (Transformation|GetWorldTransform (Variables|Default|GetItem)) "Undefined" 0 0))