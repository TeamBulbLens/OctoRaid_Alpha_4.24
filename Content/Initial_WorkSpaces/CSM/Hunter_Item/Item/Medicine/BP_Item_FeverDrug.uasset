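; BP_Item_FeverDrug is a pickup item that spins every tick and grants an effect on overlap, then destroys itself.
; Overlap casts the other actor to two classes: BP_PlayerCharacter_SN receives JumpBuffsOn, while BP_MotionControllerMain receives OctoFever.
; Disconnected nodes hold unused speed-buff setup, buff debug and FeverSys calls, so despite the name the player character gets only the jump buff call.
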(event EventBeginPlay)

(event Collision|EventActorBeginOverlap
  (params (OtherActor :type Actor%20Object%20Reference))
  (Utilities|FlowControl|Sequence
    (:then_0
      (bind _asbp_player_character_sn (Utilities|Casting|CastToBP_PlayerCharacter_SN OtherActor))
      (Default|JumpBuffson _asbp_player_character_sn)
      (Actor|DestroyActor))
    (:then_1
      (bind _asbp_motion_controller_main (Utilities|Casting|CastToBP_MotionControllerMain OtherActor))
      (Default|OctoFever _asbp_motion_controller_main)
      (Actor|DestroyActor))))

(event EventTick
  (params (DeltaSeconds :type Float%20%28single-precision%29))
  (Transformation|AddActorLocalRotation (* "0,200.000000, 0" (Utilities|Time|GetWorldDeltaSeconds)) false false))

(fn ConstructionScript)