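; BP_Item_SpeedDrug is a speed-boost medicine pickup that spins in place until a player touches it.
; Tick rotates it around yaw at a frame-rate-independent rate.
; On overlap with BP_PlayerCharacter_SN, it copies its buff percent and duration into the character, calls that character's SpeedBuffs, then destroys itself.
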(event EventBeginPlay)

(event Collision|EventActorBeginOverlap
  (params (OtherActor :type Actor%20Object%20Reference))
  (bind _asbp_player_character_sn (Utilities|Casting|CastToBP_PlayerCharacter_SN OtherActor))
  (Utilities|FlowControl|Sequence
    (:then_0
      (Variables|/Game/Blueprints/SN/Blueprints_SN/BP_PlayerCharacter_SN.BP_PlayerCharacter_SN_C|SetBuffsEffectPercentSet _asbp_player_character_sn (Variables|Default|GetBuffEffectPercent))
      (Variables|/Game/Blueprints/SN/Blueprints_SN/BP_PlayerCharacter_SN.BP_PlayerCharacter_SN_C|SetBuffsEndDelay _asbp_player_character_sn (Variables|Default|GetBufftime)))
    (:then_1
      (Default|SpeedBuffs _asbp_player_character_sn)
      (Actor|DestroyActor))))

(event EventTick
  (params (DeltaSeconds :type Float%20%28single-precision%29))
  (Transformation|AddActorLocalRotation (* "0,200.000000, 0" (Utilities|Time|GetWorldDeltaSeconds)) false false))

(fn ConstructionScript)