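; BP_Item_Bullet is an ammo pickup that gives ammo to the player on overlap.
; Shortly after BeginPlay, a delay activates its particle system.
; Overlap with BP_PlayerCharacter_SN calls the player's GetAmmo and sets SendAmmo, which lets the second Sequence branch destroy the item.
; A spin animation exists but is disconnected from Tick, so the pickup does not rotate through this graph.
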(event EventBeginPlay
  ;[1 1 1] ParticleSystem 활성화
  (Utilities|FlowControl|Delay 0.2)
  (Components|Activation|SetActive (Variables|Default|GetParticleSystem) true false))

(event Collision|EventActorBeginOverlap
  (params (OtherActor :type Actor%20Object%20Reference))
  ;[1 1 1] SendAmmo
  (Utilities|FlowControl|Sequence
    (:then_0
      (bind _asbp_player_character_sn (Utilities|Casting|CastToBP_PlayerCharacter_SN OtherActor))
      (Default|GetAmmo _asbp_player_character_sn)
      (Variables|Default|SetSendAmmo? true))
    (:then_1
      (if (Variables|Default|GetSendAmmo?)
        (Actor|DestroyActor)))))

(event EventTick
  (params (DeltaSeconds :type Float%20%28single-precision%29))
  ;[1 1 1] Item 회전 애니
)

(fn ConstructionScript)