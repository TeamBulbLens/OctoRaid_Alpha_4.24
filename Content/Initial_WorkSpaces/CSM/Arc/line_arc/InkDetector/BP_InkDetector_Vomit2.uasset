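; BP_InkDetector_Vomit2 is an ink detector actor that inflicts a vomit debuff on the player who touches it.
; When its HitCollision overlaps a BP_PlayerCharacter_SN, it writes effect percent, duration and auto-off settings into the character's buff variables.
; It then sets fixed damage and tick-interval values and calls Vomitsys on the character, which handles the effect itself.
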(event OnComponentBeginOverlap(HitCollision)
  (params (OverlappedComponent :type Primitive%20Component%20Object%20Reference) (OtherActor :type Actor%20Object%20Reference) (OtherComp :type Primitive%20Component%20Object%20Reference) (OtherBodyIndex :type Integer) (bFromSweep :type Boolean) (SweepResult :type Hit%20Result%20Structure%20%28by%20ref%29))
  (bind _asbp_player_character_sn (Utilities|Casting|CastToBP_PlayerCharacter_SN OtherActor))
  (Utilities|FlowControl|Sequence
    (:then_0
      (Variables|/Game/Blueprints/SN/Blueprints_SN/BP_PlayerCharacter_SN.BP_PlayerCharacter_SN_C|SetBuffsEffectPercentSet _asbp_player_character_sn (Variables|Default|GetBuffEffectPercent))
      (Variables|/Game/Blueprints/SN/Blueprints_SN/BP_PlayerCharacter_SN.BP_PlayerCharacter_SN_C|SetBuffsEndDelay _asbp_player_character_sn (Variables|Default|GetDebuffTime))
      (Variables|/Game/Blueprints/SN/Blueprints_SN/BP_PlayerCharacter_SN.BP_PlayerCharacter_SN_C|SetBuffsAutoOff _asbp_player_character_sn true)
      (Variables|/Game/Blueprints/SN/Blueprints_SN/BP_PlayerCharacter_SN.BP_PlayerCharacter_SN_C|SetUseBuffEndDelay? _asbp_player_character_sn true))
    (:then_1
      (Variables|/Game/Blueprints/SN/Blueprints_SN/BP_PlayerCharacter_SN.BP_PlayerCharacter_SN_C|SetResultDamage _asbp_player_character_sn 2e+01)
      (Variables|/Game/Blueprints/SN/Blueprints_SN/BP_PlayerCharacter_SN.BP_PlayerCharacter_SN_C|SetTickDamageTime _asbp_player_character_sn 0.5))
    (:then_2
      (Default|Vomitsys _asbp_player_character_sn))))

(event EventBeginPlay
  (|CallParentFunction) ; 지금 이 노드는 비활성 상태입니다. \n핀을 끌어서 다른 노드를 연결하면 활성화됩니다.
)

(event Collision|EventActorBeginOverlap
  (params (OtherActor :type Actor%20Object%20Reference))
  (|CallParentFunction OtherActor) ; 지금 이 노드는 비활성 상태입니다. \n핀을 끌어서 다른 노드를 연결하면 활성화됩니다.
)

(event EventTick
  (params (DeltaSeconds :type Float%20%28single-precision%29))
  (|CallParentFunction DeltaSeconds) ; 지금 이 노드는 비활성 상태입니다. \n핀을 끌어서 다른 노드를 연결하면 활성화됩니다.
)

(fn ConstructionScript
  (|CallParentFunction))