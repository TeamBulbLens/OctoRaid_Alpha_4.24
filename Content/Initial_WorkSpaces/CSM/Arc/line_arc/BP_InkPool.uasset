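; BP_InkPool is a short-lived ink pool hazard that slows BP_PlayerCharacter_SN players standing in it and destroys itself after ten seconds.
; On BeginPlay a looping timer calls ScaleUP to widen the pool horizontally in steps.
; HitBox overlap sets the player's buff percentage and turns on the slow debuff; leaving sets an end delay and turns it off.
; ScaleUP's step limit calls UnPauseTimer, so it never halts growth.
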(event OnComponentBeginOverlap(HitBox)
  (params (OverlappedComponent :type Primitive%20Component%20Object%20Reference) (OtherActor :type Actor%20Object%20Reference) (OtherComp :type Primitive%20Component%20Object%20Reference) (OtherBodyIndex :type Integer) (bFromSweep :type Boolean) (SweepResult :type Hit%20Result%20Structure%20%28by%20ref%29))
  (bind _asbp_player_character_sn (Utilities|Casting|CastToBP_PlayerCharacter_SN OtherActor))
  (Utilities|FlowControl|Sequence
    (:then_0
      (Variables|/Game/Blueprints/SN/Blueprints_SN/BP_PlayerCharacter_SN.BP_PlayerCharacter_SN_C|SetBuffsEffectPercentSet _asbp_player_character_sn (Variables|Default|GetBuffEffectPercent)))
    (:then_1
      (Default|SlowDebuffson _asbp_player_character_sn))))

(event OnComponentEndOverlap(HitBox)
  (params (OverlappedComponent :type Primitive%20Component%20Object%20Reference) (OtherActor :type Actor%20Object%20Reference) (OtherComp :type Primitive%20Component%20Object%20Reference) (OtherBodyIndex :type Integer))
  (bind _asbp_player_character_sn (Utilities|Casting|CastToBP_PlayerCharacter_SN OtherActor))
  (Utilities|FlowControl|Sequence
    (:then_0
      (Variables|/Game/Blueprints/SN/Blueprints_SN/BP_PlayerCharacter_SN.BP_PlayerCharacter_SN_C|SetUseBuffEndDelay? _asbp_player_character_sn true)
      (Variables|/Game/Blueprints/SN/Blueprints_SN/BP_PlayerCharacter_SN.BP_PlayerCharacter_SN_C|SetBuffsEndDelay _asbp_player_character_sn 3.0))
    (:then_1
      (Default|SlowDebuffsOff _asbp_player_character_sn))))

(event Custom|MultiScaleUP
  (Utilities|Time|SetTimerbyFunctionName 0 "ScaleUP" (Variables|Default|GetSetTimer) true))

(event Custom|SurverScaleUP
  (CallFunction|MultiScaleUP))

(event EventBeginPlay
  (Actor|SetLifeSpan 1e+01)
  (CallFunction|SurverScaleUP))

(event Collision|EventActorBeginOverlap
  (params (OtherActor :type Actor%20Object%20Reference)))

(fn ConstructionScript)

(fn Default)

(fn ScaleUP
  (Transformation|SetActorScale3D (+ (Transformation|GetActorScale3D) "1.000000,1.000000,0.000000"))
  (Variables|Default|SetTimer (+ (Variables|Default|GetTimer) 1.0))
  (if (== (Variables|Default|GetTimer) 2e+01)
    (Class|KismetSystemLibrary|UnPauseTimer 0 "ScaleUP")))