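; BP_ClimbableWall is a VR climbable wall that lets the player pull their pawn along by gripping with motion controllers.
; Climbing and Letgo track up to two gripping controllers, anchoring a pivot at the newest grip or at the remaining hand after release.
; While gripped, Tick offsets the pawn by the active controller's drift from that pivot, then pins the controller back onto it.
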(event Custom|UpdateLog
  (bind _firstmotioncontroller (Variables|Default|GetFirstMotionController))
  (bind _secondmotioncontroller (Variables|Default|GetSecondMotionController))
  ;[1 1 0] 코멘트
  (Rendering|Components|TextRender|SetText (Variables|Default|GetTextRender) (Utilities|Text|ToText(String) (Utilities|String|Append (select (Utilities|IsValid _firstmotioncontroller) (Utilities|GetDisplayName _firstmotioncontroller) "None") " " (select (Utilities|IsValid _secondmotioncontroller) (Utilities|GetDisplayName _secondmotioncontroller) "None")))))

(event EventTick
  (params (DeltaSeconds :type Float%20%28single-precision%29))
  (bind _firstmotioncontroller (Variables|Default|GetFirstMotionController))
  (bind _secondmotioncontroller (Variables|Default|GetSecondMotionController))
  (bind _firstmotioncontroller_2 (Variables|Default|GetFirstMotionController))
  (bind _secondmotioncontroller_2 (Variables|Default|GetSecondMotionController))
  ;[1 1 1] tick
  (|CallParentFunction DeltaSeconds)
  (Utilities|IsValid (Variables|Default|GetVRPawn)
    (:Is%20Valid
      (if (Variables|Default|GetIsUsing)
        (Utilities|IsValid (Variables|Default|GetFirstMotionController)
          (:Is%20Valid
            (Utilities|IsValid (Variables|Default|GetSecondMotionController)
              (:Is%20Valid
                (Transformation|AddActorWorldOffset (Variables|Default|GetVRPawn) (- (Variables|Default|GetPivotPoint) (Transformation|GetWorldLocation _secondmotioncontroller)))
                (Transformation|SetWorldLocation _secondmotioncontroller (Variables|Default|GetPivotPoint) false false))
              (:Is%20Not%20Valid
                (Transformation|AddActorWorldOffset (Variables|Default|GetVRPawn) (- (Variables|Default|GetPivotPoint) (Transformation|GetWorldLocation _firstmotioncontroller)))
                (Transformation|SetWorldLocation _firstmotioncontroller (Variables|Default|GetPivotPoint) false false)))))
        (else
          ;;[1 1 1] 현재 붙잡고 있는 상태가 아니면 놓기
          (Utilities|IsValid _secondmotioncontroller_2
            (:Is%20Valid
              (CallFunction|Letgo _secondmotioncontroller_2))
            (:Is%20Not%20Valid
              _))
          (Utilities|IsValid _firstmotioncontroller_2
            (:Is%20Valid
              (CallFunction|Letgo _firstmotioncontroller_2))))))))

(event EventClimbing
  (params (Motion%20Controller :type Scene%20Component%20Object%20Reference))
  ;[1 1 1] climbing
  (Utilities|IsValid Motion%20Controller
    (:Is%20Valid
      (Utilities|IsValid (Variables|Default|GetFirstMotionController)
        (:Is%20Valid
          (if (!= (Variables|Default|GetFirstMotionController) Motion%20Controller)
            (Variables|Default|SetSecondMotionController Motion%20Controller)
            (Variables|Default|SetPivotPoint (Transformation|GetWorldLocation (select (Utilities|IsValid (Variables|Default|GetSecondMotionController)) (Variables|Default|GetSecondMotionController) (Variables|Default|GetFirstMotionController))) :!label _label)
            (Variables|Default|SetVRPawn (Game|Player|GetPlayerPawn 0))
            (Variables|Default|SetIsUsing true)))
        (:Is%20Not%20Valid
          (Variables|Default|SetFirstMotionController Motion%20Controller)
          (goto _label))))))

(event EventLetgo
  (params (Motion%20Controller :type Scene%20Component%20Object%20Reference))
  ;[1 1 1] letgo
  (Utilities|IsValid (Variables|Default|GetSecondMotionController)
    (:Is%20Valid
      (if (== Motion%20Controller (Variables|Default|GetSecondMotionController))
        (Variables|Default|SetSecondMotionController 0)
        (Variables|Default|SetPivotPoint (Transformation|GetWorldLocation (Variables|Default|GetFirstMotionController)))
        (else
          (Variables|Default|SetFirstMotionController (Variables|Default|GetSecondMotionController))
          (Variables|Default|SetSecondMotionController 0)
          (Variables|Default|SetPivotPoint (Transformation|GetWorldLocation (Variables|Default|GetFirstMotionController))))))
    (:Is%20Not%20Valid
      (if (== Motion%20Controller (Variables|Default|GetFirstMotionController))
        (Variables|Default|SetFirstMotionController 0)
        (Variables|Default|SetSecondMotionController 0)
        (Variables|Default|SetPivotPoint "0, 0, 0")
        (Variables|Default|SetVRPawn 0)
        (Variables|Default|SetIsUsing false)))))

(fn ConstructionScript)