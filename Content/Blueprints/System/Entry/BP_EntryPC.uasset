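; Player controller for the game's entry stage, which assigns the device role and runs the startup logo or error screen.
; Its construction script sets the BP_GI role from local headset connection, Android platform or any other platform.
; On BeginPlay, Octopus instances wait the logo time before calling ReadyForGame.
; Others branch on game state: Ready adds the entry widget before that same wait, while Network Error shows an error widget and mouse cursor.
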(event EventBeginPlay
  (bind _asbp_gi (Utilities|Casting|CastToBP_GI (Game|GetGameInstance)))
  (Utilities|IsValid _asbp_gi
    (:Is%20Valid
      (Variables|Default|SetGameInstance _asbp_gi)
      (bind _isoctopus (Default|IsOctopus _asbp_gi))
      (if _isoctopus
        ;[1 1 1] 로고 표시시간
        (Utilities|FlowControl|Delay (Variables|/Game/Blueprints/Public/BP_GI.BP_GI_C|GetLogoTime (Variables|Default|GetGameInstance)) :!label _label)
        (Default|ReadyforGame (Variables|Default|GetGameInstance))
        (else
          (switch Utilities|FlowControl|Switch|SwitchonEGameState (Variables|/Script/OctoPrototype.MyGameInstance|GetCurrentState _asbp_gi)
            (:Ready
              (bind _returnvalue (UserInterface|CreateWidget "/Game/Blueprints/System/Entry/EntryWidget.EntryWidget_C"))
              (UserInterface|Viewport|AddtoViewport _returnvalue 0)
              (goto _label))
            (:NetworkError
              (bind _returnvalue_2 (UserInterface|CreateWidget "/Game/Blueprints/System/Entry/NetworkErrorWidget.NetworkErrorWidget_C"))
              (UserInterface|Viewport|AddtoViewport _returnvalue_2 0)
              (Variables|Default|SetbShowMouseCursor true))))))))

(event EventTick
  (params (DeltaSeconds :type Float%20%28single-precision%29)))

(fn ConstructionScript
  (bind _returnvalue (Game|GetPlatformName))
  (bind _asbp_gi (Utilities|Casting|CastToBP_GI (Game|GetGameInstance)))
  (Utilities|IsValid _asbp_gi
    (:Is%20Valid
      (if (and (Pawn|IsLocalPlayerController) (Class|HeadMountedDisplayFunctionLibrary|IsHeadMountedDisplayConnected))
        (Default|SetGIRoleState _asbp_gi "NewEnumerator0")
        (elif (Utilities|Enum|Equal(Enum) _returnvalue "Android")
          (Default|SetGIRoleState _asbp_gi "NewEnumerator2")
          (Development|PrintString _returnvalue true true "(R=0.000000,G=0.660000,B=1.000000,A=1.000000)" 3e+01)
          (else
            (Default|SetGIRoleState _asbp_gi "NewEnumerator1")
            (Development|PrintString _returnvalue true true "(R=0.000000,G=0.660000,B=1.000000,A=1.000000)" 3e+01)))))))