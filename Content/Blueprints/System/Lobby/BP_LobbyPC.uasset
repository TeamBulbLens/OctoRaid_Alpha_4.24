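; Lobby player controller for a VR octopus-versus-hunters game, setting the role at construction from local headset detection.
; Non-octopus players get lobby (debug-mode server) or hunter-control (client) widgets, using GameMode validity as the server check.
; GameStart attaches a countdown to the VR camera, triggers hunters' countdown and loading screens, and calls the GameInstance to start the match.
; Other events relay PlayerState info and skins; debug keys print them.
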(event Custom|GameStart
  ;[1 1 1] 게임맵으로 이동
  (Utilities|FlowControl|Sequence
    (:then_0
      ;;[1 1 1] Octo에 카운트다운 위젯을 붙인다
      (Utilities|IsValid (Game|GetGameMode)
        (:Is%20Valid
          (bind _asbp_vrpawn_main (Utilities|Casting|CastToBP_VRPawnMain (Pawn|GetControlledPawn)))
          (Utilities|IsValid _asbp_vrpawn_main
            (:Is%20Valid
              (bind _returnvalue (Game|SpawnActorfromClass "/Game/Blueprints/System/Lobby/BP_CountdownWidget.BP_CountdownWidget_C" (Transformation|GetWorldTransform (Variables|/Game/Blueprints/Octopus/BP_VRPawnMain.BP_VRPawnMain_C|GetCamera _asbp_vrpawn_main)) "Undefined" _asbp_vrpawn_main 0))
              (Transformation|AttachComponentToComponent _returnvalue (Variables|/Game/Blueprints/Octopus/BP_VRPawnMain.BP_VRPawnMain_C|GetCamera _asbp_vrpawn_main) "None" "KeepWorld" "KeepWorld" "KeepWorld" true))))))
    (:then_1
      ;;[1 1 1] 헌터들에게 카운트다운 표시
      (Utilities|IsValid (Game|GetGameMode)
        (:Is%20Valid
          (bind _outactors (Actor|GetAllActorsOfClass "BP_LobbyPC_C"))
          (for _array_element _outactors
            (CallFunction|ShowCountdown _array_element)))))
    (:then_2
      (bind _asbp_gi (Utilities|Casting|CastToBP_GI (Game|GetGameInstance)))
      (Default|StartMainGame _asbp_gi 3.0))))

(event Custom|ShowLoading
  ;[1 1 1] 게임맵으로 이동
  ;;[1 1 1] 로딩화면 표시 (client)
  (if (and (Pawn|IsLocalController) (Utilities|Enum|Equal(Enum) (Variables|Default|GetRoleState) "NewEnumerator1"))
    (Viewport|RemoveAllWidgets)
    (bind _returnvalue (UserInterface|CreateWidget "/Game/Blueprints/System/Public/LoadingWidget.LoadingWidget_C"))
    (UserInterface|Viewport|AddtoViewport _returnvalue 0)))

(event Custom|ShowCountdown
  (if (and (Pawn|IsLocalController) (Utilities|Enum|Equal(Enum) (Variables|Default|GetRoleState) "NewEnumerator1"))
    (Viewport|RemoveAllWidgets)
    (bind _returnvalue (UserInterface|CreateWidget "/Game/Blueprints/System/Lobby/CountdownWidget.CountdownWidget_C"))
    (UserInterface|Viewport|AddtoViewport _returnvalue 0)
    (Variables|Default|SetbShowMouseCursor false)
    (Input|SetInputModeUIOnly self 0 "DoNotLock")
    (Utilities|FlowControl|Delay 3.0)
    (CallFunction|ShowLoading)))

(event Custom|SetLocalInfoToClients
  (Utilities|IsValid (Game|GetGameMode)
    (:Is%20Valid
      (Utilities|FlowControl|Delay 2.0)
      (bind _outactors (Actor|GetAllActorsOfClass "/Game/Blueprints/System/Lobby/BP_LobbyPS.BP_LobbyPS_C"))
      (for _array_element _outactors
        (Default|SetLocalInfotoClientGI _array_element)))))

(event Custom|SetMeshAndMatServer
  (bind _outactors (Actor|GetAllActorsOfClass "/Game/Blueprints/System/Lobby/BP_LobbyPS.BP_LobbyPS_C"))
  (for _array_element _outactors
    (Default|SetMeshandMaterial _array_element)))

(event EventBeginPlay
  ;[1 1 1] 초기화
  (bind _isoctopus (CallFunction|IsOctopusLobbyPC))
  (if (not _isoctopus)
    ;;[1 1 1] Is Android 추가 부분
    (bind _is_android (CallFunction|IsAndroidLobbyPC))
    (if _is_android
      _
      (else
        _))
    (Utilities|FlowControl|Sequence
      (:then_0
        ;;[1 0.9853 0] 헌터가 server일 경우
        (bind _asbp_gi (Utilities|Casting|CastToBP_GI (Game|GetGameInstance)))
        (if (Variables|/Game/Blueprints/Public/BP_GI.BP_GI_C|GetIsDebugMode _asbp_gi)
          (Utilities|IsValid (Game|GetGameMode)
            (:Is%20Valid
              (bind _returnvalue (UserInterface|CreateWidget "/Game/Blueprints/System/Lobby/LobbyWidget.LobbyWidget_C"))
              (UserInterface|Viewport|AddtoViewport _returnvalue 0)
              (Variables|Default|SetbShowMouseCursor true)
              (Input|SetInputModeGameandUI self 0 "DoNotLock" true)))))
      (:then_1
        (Utilities|IsValid (Game|GetGameMode)
          (:Is%20Not%20Valid
            (bind _returnvalue_2 (UserInterface|CreateWidget "/Game/Blueprints/HunterUI/HunterControlWidget.HunterControlWidget_C"))
            (UserInterface|Viewport|AddtoViewport _returnvalue_2 0)))))))

(event Input|KeyboardEvents|F1
  (params (Key :type Key%20Structure :default "None"))
  ;[1 0.8557 0] for debug
  (:Pressed
    (bind _asbp_gi (Utilities|Casting|CastToBP_GI (Game|GetGameInstance)))
    (Variables|/Game/Blueprints/Public/BP_GI.BP_GI_C|SetIsDebugMode _asbp_gi (not (Variables|/Game/Blueprints/Public/BP_GI.BP_GI_C|GetIsDebugMode _asbp_gi)))))

(event Input|KeyboardEvents|P
  (params (Key :type Key%20Structure :default "None"))
  ;[1 0.8557 0] for debug
  (:Pressed
    (bind _asbp_gi (Utilities|Casting|CastToBP_GI (Game|GetGameInstance)))
    (if true
      (Development|PrintString (Utilities|String|Append "UID : " (Utilities|String|ToString(Integer) (Variables|/Game/Blueprints/Public/BP_GI.BP_GI_C|GetLocalUID _asbp_gi)) " SKin : " (Utilities|String|EnumtoString (Variables|/Game/Blueprints/Public/BP_GI.BP_GI_C|GetLocalSkinState _asbp_gi))) true true "(R=1.000000,G=0.124706,B=0.000000,A=1.000000)" 12.0))))

(event Input|KeyboardEvents|I
  (params (Key :type Key%20Structure :default "None"))
  ;[1 0.8557 0] for debug
  (:Pressed
    (bind _asbp_gi (Utilities|Casting|CastToBP_GI (Game|GetGameInstance)))
    (if (Variables|/Game/Blueprints/Public/BP_GI.BP_GI_C|GetIsDebugMode _asbp_gi)
      (bind _asbp_lobby_ps (Utilities|Casting|CastToBP_LobbyPS (Variables|GetPlayerState)))
      (Development|PrintString (Utilities|String|Append "UID : " (Utilities|String|ToString(Integer) (Variables|/Game/Blueprints/System/Lobby/BP_LobbyPS.BP_LobbyPS_C|GetUID _asbp_lobby_ps)) " SKin : " (Utilities|String|EnumtoString (Variables|/Game/Blueprints/System/Lobby/BP_LobbyPS.BP_LobbyPS_C|GetLocalSkinState _asbp_lobby_ps))) true true "(R=0.000000,G=1.000000,B=0.052316,A=1.000000)" 12.0))))

(fn ConstructionScript
  (if (and (Pawn|IsLocalController) (Class|HeadMountedDisplayFunctionLibrary|IsHeadMountedDisplayConnected))
    (Variables|Default|SetRoleState "NewEnumerator0")
    (else
      (Variables|Default|SetRoleState "NewEnumerator1"))))

(fn IsOctopusLobbyPC
  (return (Utilities|Enum|Equal(Enum) (Variables|Default|GetRoleState) "NewEnumerator0")))

(fn IsAndroidLobbyPC
  (return (Utilities|Enum|Equal(Enum) (Variables|Default|GetRoleState) "NewEnumerator2")))