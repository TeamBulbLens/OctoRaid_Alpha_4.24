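; Lobby game mode that registers joining players and spawns them as either a VR Octopus or a hunter.
; PostLogin takes a UID and skin from BP_GI, copies them to BP_LobbyPS (and to BP_GI for the host, who also sorts skins), then possesses the spawned pawn.
; Start points come from actor tags, with hunters indexed by UID.
; A debug flag forces UID 0 to Octo; logout frees the UID.
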(event EventOnLogout
  (params (ExitingController :type Controller%20Object%20Reference))
  ;[1 1 1] 로그아웃하면 UID 인덱스를 사용할 수 있게 리스트에서 비운다
  (bind _asbp_lobby_ps (Utilities|Casting|CastToBP_LobbyPS (Variables|/Script/Engine.Controller|GetPlayerState ExitingController)))
  (Utilities|IsValid _asbp_lobby_ps
    (:Is%20Valid
      (bind _asbp_gi (Utilities|Casting|CastToBP_GI (Game|GetGameInstance)))
      (Utilities|IsValid _asbp_gi
        (:Is%20Valid
          (Default|SetUIDEmpty _asbp_gi (Variables|/Game/Blueprints/System/Lobby/BP_LobbyPS.BP_LobbyPS_C|GetUID _asbp_lobby_ps)))))))

(event EventPostLogin
  (params (NewPlayer :type Player%20Controller%20Object%20Reference))
  (bind _asbp_gi (Utilities|Casting|CastToBP_GI (Game|GetGameInstance)))
  (Utilities|IsValid _asbp_gi
    (:Is%20Valid
      (bind _uid (Default|GetUID _asbp_gi))
      (bind _output_get (Variables|Default|SetPlayerIndex _uid))
      ;[1 1 1] GameInstance에서 이 옵션이 켜져 있으면 첫번째 플레이어는 Octo로 나온다
      (if (Variables|/Game/Blueprints/Public/BP_GI.BP_GI_C|GetDebugUID0IsOcto _asbp_gi)
        (if (== _output_get 0)
          (bind _asbp_lobby_pc (Utilities|Casting|CastToBP_LobbyPC NewPlayer))
          (Variables|/Game/Blueprints/System/Lobby/BP_LobbyPC.BP_LobbyPC_C|SetRoleState _asbp_lobby_pc "NewEnumerator0")))
      (CallFunction|SortSkinList NewPlayer)
      (bind _skinstate (CallFunction|GetSkin (Variables|Default|GetPlayerIndex)))
      (CallFunction|SetLocalInfotoServer NewPlayer (Variables|Default|GetPlayerIndex) _skinstate)
      (CallFunction|SetUserInfotoPS NewPlayer (Variables|Default|GetPlayerIndex) _skinstate)
      (bind _asbp_lobby_pc_2 (Utilities|Casting|CastToBP_LobbyPC NewPlayer))
      ;[1 1 1] 코멘트
      (bind _isoctopus (Default|IsOctopusLobbyPC _asbp_lobby_pc_2))
      (bind _output (CallFunction|GetStartPoint NewPlayer))
      (bind _returnvalue (Game|SpawnActorfromClass (select _isoctopus "/Game/Blueprints/Octopus/BP_VRPawnMain.BP_VRPawnMain_C" "/Game/Blueprints/SN/Blueprints_SN/BP_PlayerCharacter_SN.BP_PlayerCharacter_SN_C") (Transformation|GetActorTransform _output) "AlwaysSpawn" 0 0))
      (bind _aspawn (Utilities|Casting|CastToPawn _returnvalue))
      (Pawn|Possess NewPlayer _aspawn)
      (bind _asbp_lobby_pc_3 (Utilities|Casting|CastToBP_LobbyPC NewPlayer))
      (Utilities|IsValid _asbp_lobby_pc_3
        (:Is%20Valid
          (Default|SetLocalInfotoClients _asbp_lobby_pc_3))))))

(fn ConstructionScript)

(fn GetStartPoint
  (params (Object :type Player%20Controller%20Object%20Reference))
  (bind _asbp_lobby_pc (Utilities|Casting|CastToBP_LobbyPC Object))
  (bind _isoctopus (Default|IsOctopusLobbyPC _asbp_lobby_pc))
  (if _isoctopus
    ;[1 1 1] VR시작위치
    (Variables|Default|SetIsOctoServer (and (== (Variables|Default|GetPlayerIndex) 0) _isoctopus))
    (bind _outactors (Actor|GetAllActorswithTag "OctoStart"))
    (return (Utilities|Array|Get(acopy) _outactors))
    (else
      ;[1 1 1] 헌터 시작위치
      (if (== (Utilities|Array|Length (Variables|Default|GetHunterSpawnPoints)) 0)
        (bind _outactors_2 (Actor|GetAllActorswithTag "HunterStart"))
        (Variables|Default|SetHunterSpawnPoints _outactors_2))
      (if (Variables|Default|GetIsOctoServer)
        (return (Utilities|Array|Get(acopy) (Variables|Default|GetHunterSpawnPoints) (- (Utilities|Array|Length (Variables|Default|GetHunterSpawnPoints)) (Variables|Default|GetPlayerIndex))))
        (else
          (return (Utilities|Array|Get(acopy) (Variables|Default|GetHunterSpawnPoints) (- (- (Utilities|Array|Length (Variables|Default|GetHunterSpawnPoints)) 1) (Variables|Default|GetPlayerIndex)))))))))

(fn SortSkinList
  (params (NewPlayer :type Player%20Controller%20Object%20Reference))
  ;[1 1 1] 서버에서 한번만 실행
  (if (Pawn|IsLocalController NewPlayer)
    (bind _asbp_gi (Utilities|Casting|CastToBP_GI (Game|GetGameInstance)))
    (Utilities|IsValid _asbp_gi
      (:Is%20Valid
        (Default|SortSkinList _asbp_gi))))
  (return))

(fn GetSkin
  (params (UID :type Integer))
  (bind _asbp_gi (Utilities|Casting|CastToBP_GI (Game|GetGameInstance)))
  (Utilities|IsValid _asbp_gi
    (:Is%20Valid
      (bind _skinstate (Default|GetSkin _asbp_gi UID))
      (return _skinstate))))

(fn SetLocalInfotoServer
  (params (NewPlayer :type Player%20Controller%20Object%20Reference) (UID :type Integer) (SkinState :type ESkinState%20Enum :default "NewEnumerator0"))
  ;[1 1 1] 서버일때만 한번 실행
  (if (Pawn|IsLocalPlayerController NewPlayer)
    (bind _asbp_gi (Utilities|Casting|CastToBP_GI (Game|GetGameInstance)))
    (Utilities|IsValid _asbp_gi
      (:Is%20Valid
        (Default|SetLocalSkinState _asbp_gi SkinState)
        (Default|SetLocalUID _asbp_gi UID))))
  (return))

(fn SetUserInfotoPS
  (params (NewPlayer :type Player%20Controller%20Object%20Reference) (UID :type Integer) (SkinState :type ESkinState%20Enum :default "NewEnumerator0"))
  (bind _asbp_lobby_pc (Utilities|Casting|CastToBP_LobbyPC NewPlayer))
  (Utilities|IsValid _asbp_lobby_pc
    (:Is%20Valid
      (bind _asbp_lobby_ps (Utilities|Casting|CastToBP_LobbyPS (Variables|/Script/Engine.Controller|GetPlayerState _asbp_lobby_pc)))
      (Utilities|IsValid _asbp_lobby_ps
        (:Is%20Valid
          (Default|SetUID _asbp_lobby_ps UID)
          (Default|SetLocalSkinState _asbp_lobby_ps SkinState))))))